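; BP_Turret is a turret that fires while the player is inside its room, driven by RoomController enter and exit bindings.
; A single timeline animates gun recoil by lerping the mesh's relative location and spawns BP_TurretBullet at the Scene component's transform from its Shoot event track.
; Exiting the room stops the timeline, and the construction script sets its play rate from ShootTimeRate to control firing speed.
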(event Custom|Shoot
  (bind _newtrack_0 (Timeline|ShootTimeline Play)
    (:Update
      (Transformation|SetRelativeLocation (Variables|Default|GetSM_TurretGun) (Math|Vector|Lerp(Vector) "90.000000,0.000000,0.000000" "50.000000,0.000000,0.000000" _newtrack_0) false false))
    (:Shoot
      (Game|SpawnActorfromClass "/Game/InteractionObjects/Turret/Blueprints/BP_TurretBullet.BP_TurretBullet_C" (Transformation|GetWorldTransform (Variables|Default|GetScene)) "Undefined" "MultiplyWithRoot" 0 0))))

(event Custom|StopShoot
  (bind _newtrack_0 (Timeline|ShootTimeline Stop)
    (:Update
      (Transformation|SetRelativeLocation (Variables|Default|GetSM_TurretGun) (Math|Vector|Lerp(Vector) "90.000000,0.000000,0.000000" "50.000000,0.000000,0.000000" _newtrack_0) false false))
    (:Shoot
      (Game|SpawnActorfromClass "/Game/InteractionObjects/Turret/Blueprints/BP_TurretBullet.BP_TurretBullet_C" (Transformation|GetWorldTransform (Variables|Default|GetScene)) "Undefined" "MultiplyWithRoot" 0 0))))

(event EventBeginPlay
  (bind _roomcontroller (Variables|Default|GetRoomController))
  (EventDispatchers|BindEventtoPlayerEnterinRoom _roomcontroller (delegate Custom|Shoot))
  (EventDispatchers|BindEventtoPlayerExitfromRoom _roomcontroller (delegate Custom|StopShoot)))

(fn ConstructionScript
  (Components|Timeline|SetPlayRate (Variables|Default|GetShootTimeline) (Variables|Default|GetShootTimeRate)))