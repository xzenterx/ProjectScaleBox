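; BP_RoomController is a level actor that tracks whether the player character is inside a room.
; Separate enter and exit trigger components respond to BP_Character overlaps by calling PlayerEnterInRoom or PlayerExitFromRoom and updating IsPlayerInRoom.
; The construction script positions both triggers from location variables, so each placed room can set its own entry and exit points.
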(event OnComponentBeginOverlap(EnterRoomTriger)
  (params (OverlappedComponent :type Primitive%20Component%20Object%20Reference) (OtherActor :type Actor%20Object%20Reference) (OtherComp :type Primitive%20Component%20Object%20Reference) (OtherBodyIndex :type Integer) (bFromSweep :type Boolean) (SweepResult :type Hit%20Result%20Structure%20%28by%20ref%29))
  (Utilities|Casting|CastToBP_Character OtherActor)
  (Default|CallPlayerEnterinRoom)
  (Variables|Default|SetIsPlayerInRoom true))

(event OnComponentBeginOverlap(ExitRoomTriger)
  (params (OverlappedComponent :type Primitive%20Component%20Object%20Reference) (OtherActor :type Actor%20Object%20Reference) (OtherComp :type Primitive%20Component%20Object%20Reference) (OtherBodyIndex :type Integer) (bFromSweep :type Boolean) (SweepResult :type Hit%20Result%20Structure%20%28by%20ref%29))
  (Utilities|Casting|CastToBP_Character OtherActor)
  (Default|CallPlayerExitfromRoom)
  (Variables|Default|SetIsPlayerInRoom false))

(fn ConstructionScript
  (Transformation|SetRelativeLocation (Variables|Default|GetEnterRoomTriger) (Variables|Default|GetEnterRoomTrigerLocation) false false)
  (Transformation|SetRelativeLocation (Variables|Default|GetExitRoomTriger) (Variables|Default|GetExitRoomTrigerLocation) false false))